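; BP_NPC is a non-player character that the player can talk to through a sequence of dialogue lines.
; Each Talk call shows the next Text entry in a lazily created DialoguePanel widget and disables the player character's movement.
; A call after the last line removes the panel, resets the index and restores walking.
; The BP_ThirdPersonCharacter reference is cached on first use.
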(event `/Game/Interface/BPI_Talk.Talk`
  (bind _charactermovement (`Character.CharacterMovement` (`self.PlayerRef`)))
  (if (> (`KismetArrayLibrary.Array_Length` (`self.Text`)) (`self.Index`))
    (`/Engine/EditorBlueprintResources/StandardMacros.IsValid` (`self.PlayerRef`)
      (:`Is Valid`
        _)
      (:`Is Not Valid`
        (bind _asbp_third_person_character (cast `/Game/ThirdPerson/Blueprints/BP_ThirdPersonCharacter` (`GameplayStatics.GetPlayerCharacter` 0)))
        (set `self.PlayerRef` _asbp_third_person_character)))
    (`/Engine/EditorBlueprintResources/StandardMacros.IsValid` (`self.DIalogueUI`)
      (:`Is Valid`
        _)
      (:`Is Not Valid`
        (bind _returnvalue (`|CreateWidget` "/Game/UI/UIDesign/DialoguePanel.DialoguePanel_C"))
        (bind _output_get (set `self.DIalogueUI` _returnvalue))
        (`UserWidget.AddToPlayerScreen` _output_get 0)))
    (`TextBlock.SetText` (`/Game/UI/UIDesign/DialoguePanel.Dialogue` _output_get) (`|GetArrayItem` (`self.Text`) (`self.Index`)))
    (`CharacterMovementComponent.DisableMovement` _charactermovement)
    (`/Engine/EditorBlueprintResources/StandardMacros.IncrementInt` (`self.Index`))
    (else
      (`Widget.RemoveFromParent` (`self.DIalogueUI`))
      (set `self.Index` 0)
      (set `self.DIalogueUI` null)
      (`CharacterMovementComponent.SetMovementMode` _charactermovement "MOVE_Walking" 0))))

(fn `UserConstructionScript`)